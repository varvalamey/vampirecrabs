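; Gravity field weapon actor: a black hole with a Niagara effect that scales in on spawn and pulls in nearby physics objects.
; InfluenceExtent overlaps track simulating components, which Tick pushes toward the center by force and pins there within CaptureRadius.
; Attraction runs only while StaysActive; otherwise timelines shrink and destroy the actor.
; Helpers for saving and restoring damping and scale, and destroying enveloped actors, are defined but never called here.
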(event OnComponentEndOverlap(InfluenceExtent)
  (params (OverlappedComponent :type Primitive%20Component%20Object%20Reference) (OtherActor :type Actor%20Object%20Reference) (OtherComp :type Primitive%20Component%20Object%20Reference) (OtherBodyIndex :type Integer))
  (Utilities|Array|RemoveItem (Variables|Default|GetAffectedComponents) OtherComp))

(event OnComponentBeginOverlap(InfluenceExtent)
  (params (OverlappedComponent :type Primitive%20Component%20Object%20Reference) (OtherActor :type Actor%20Object%20Reference) (OtherComp :type Primitive%20Component%20Object%20Reference) (OtherBodyIndex :type Integer) (bFromSweep :type Boolean) (SweepResult :type Hit%20Result%20Structure%20%28by%20ref%29))
  (if (Physics|IsSimulatingPhysics OtherComp "None")
    (Utilities|Array|Add (Variables|Default|GetAffectedComponents) OtherComp)))

(event EventBeginPlay
  (Variables|InputParameters|SetAttractionActivated true)
  (bind _returnvalue (Niagara|SpawnSystemAttached "/Game/VampCrabs/Niagara/NS_Gravity.NS_Gravity" (Variables|Default|GetInfluenceExtent) "None" "0, 0, 0" "0, 0, 0" "KeepRelativeOffset" false))
  (Niagara|SetNiagaraVariable(Float) _returnvalue "SphereRadius" (Variables|Default|GetSphere%20Radius))
  (Niagara|SetNiagaraVariable(Float) _returnvalue "KillRadius" (- (Variables|Default|GetSphere%20Radius) 1e+02))
  ;[1 1 1] Black hole birth
  (bind _scale (Timeline|Timeline Play)
    (:Update
      (Transformation|SetActorScale3D self (Math|Vector|MakeVector _scale _scale _scale)))
    (:Finished
      (if (not (Variables|InputParameters|GetStaysActive))
        (Utilities|FlowControl|Delay 2.0)
        ;[1 1 1] Black hole death
        (bind _scale_2 (Timeline|BlackHoleDeath Play)
          (:Update
            (Transformation|SetActorScale3D (Math|Vector|MakeVector (- 1.0 _scale_2) (- 1.0 _scale_2) (- 1.0 _scale_2))))
          (:Finished
            (Variables|InputParameters|SetAttractionActivated false)
            (Actor|DestroyActor self)))))))

(event EventTick
  (params (DeltaSeconds :type Float%20%28single-precision%29))
  ;[1 1 1] Executes each frame
  (if (Variables|InputParameters|GetStaysActive)
    (if (Variables|InputParameters|GetAttractionActivated)
      (CallFunction|AttractComponents))
    (else
      (Variables|InputParameters|SetAttractionActivated false)
      (Utilities|FlowControl|DoOnce false
        (:Completed
          (bind _scale (Timeline|Timeline_0 Play)
            (:Update
              (Transformation|SetActorScale3D (Math|Vector|MakeVector (- 1.0 _scale) (- 1.0 _scale) (- 1.0 _scale))))
            (:Finished
              (Variables|InputParameters|SetAttractionActivated false)
              (Actor|DestroyActor self))))))))

(fn ConstructionScript)

(fn RegisterComponent
  (params (Component :type Primitive%20Component%20Object%20Reference) (Actor :type Actor%20Object%20Reference))
  (bind _affectedactors (Variables|Default|GetAffectedActors))
  (LocalVariables|SetAffectedComponent (Utilities|Struct|MakeBlackHoleAffectedComponent Component (Class|PrimitiveComponent|GetLinearDamping Component) (Class|PrimitiveComponent|GetAngularDamping Component) (Transformation|GetWorldScale Component)))
  (LocalVariables|SetOverlappedActor Actor)
  (for (_array_element _array_index) _affectedactors
    (if (== (LocalVariables|GetOverlappedActor) (.actor _array_element))
      (Utilities|Array|Add (.affectedcomponents (Utilities|Array|Get(acopy) _affectedactors _array_index)) (LocalVariables|GetAffectedComponent))
      (LocalVariables|SetFoundActor true)))
  (if (not (LocalVariables|GetFoundActor))
    (Utilities|Array|Add (Variables|Default|GetAffectedActors) (Utilities|Struct|MakeBlackHoleAffectedActor (Transformation|GetActorScale3D (LocalVariables|GetOverlappedActor)) (Utilities|Array|MakeArray (LocalVariables|GetAffectedComponent)) (LocalVariables|GetOverlappedActor)))))

(fn UnregisterComponent
  (params (ActorToUnregister :type Actor%20Object%20Reference) (ComponentToUnregister :type Actor%20Component%20Object%20Reference))
  (bind _affectedactors (Variables|Default|GetAffectedActors))
  ;[1 1 1] Find if component is registered
  (for (_array_element _array_index) _affectedactors
    (if (== ActorToUnregister (.actor _array_element))
      (for (_array_element_2 _array_index_2) (.affectedcomponents _array_element)
        (bind _asprimitive_component (Utilities|Casting|CastToPrimitiveComponent ComponentToUnregister))
        (if (== (.component _array_element_2) _asprimitive_component)
          ;[1 1 1] Component found, unregister it
          (Utilities|FlowControl|Sequence
            (:then_0
              ;;[1 1 1] Restore original damping and scale
              (Class|PrimitiveComponent|SetLinearDamping _asprimitive_component (.lineardamping _array_element_2)))
            (:then_1
              (Class|PrimitiveComponent|SetAngularDamping _asprimitive_component (.angulardamping _array_element_2)))
            (:then_2
              (Transformation|SetWorldScale3D _asprimitive_component (.originalscale _array_element_2)))
            (:then_3
              (Utilities|Array|RemoveIndex (.affectedcomponents (Utilities|Array|Get(acopy) _affectedactors _array_index)) _array_index_2))
            (:then_4
              ;;[1 1 1] Deactivate Stretch Material
              (bind _asstatic_mesh_component (Utilities|Casting|CastToStaticMeshComponent _asprimitive_component))
              (Rendering|Material|SetScalarParameterValueonMaterials _asstatic_mesh_component "StretchActivated" 0.0))))))))

(fn DestroyComponents
  (for (_array_element _array_index) (Variables|Default|GetAffectedActors)
    (LocalVariables|SetAffectedComponentsInActor (.affectedcomponents _array_element))
    (LocalVariables|SetAffectedActor (.actor _array_element))
    (LocalVariables|SetActorIndex _array_index)
    (for _array_element_2 (LocalVariables|GetAffectedComponentsInActor)
      (LocalVariables|SetComponent (.component _array_element_2))
      (if (< (/ (Math|Vector|VectorLength (- (Transformation|GetWorldLocation (Variables|/Script/Engine.Actor|GetRootComponent (LocalVariables|GetAffectedActor))) (Transformation|GetWorldLocation (Variables|Default|GetEnvelopedExtent)))) (Components|Sphere|GetScaledSphereRadius (Variables|Default|GetEnvelopedExtent))) 0.5)
        (Actor|DestroyActor (LocalVariables|GetAffectedActor))
        (Utilities|Array|RemoveIndex (Variables|Default|GetAffectedActors) (LocalVariables|GetActorIndex)))))
  (return))

(fn AttractComponents
  (for _array_element (Variables|Default|GetAffectedComponents)
    (Utilities|IsValid _array_element
      (:Is%20Valid
        (LocalVariables|SetAttractedComponent _array_element)
        (bind _output_get (LocalVariables|SetDistanceToCenter (Math|Vector|VectorLength (- (Transformation|GetActorLocation) (Transformation|GetWorldLocation _array_element)))))
        (bind _output_get_2 (LocalVariables|SetDirectionTowardsCenter (- (Transformation|GetActorLocation) (Transformation|GetWorldLocation _array_element))))
        (if (<= _output_get (Variables|InputParameters|GetCaptureRadius))
          (Physics|SetPhysicsLinearVelocity (LocalVariables|GetAttractedComponent) "0, 0, 0" false "None")
          (Class|PrimitiveComponent|SetPhysicsAngularVelocityinRadians (LocalVariables|GetAttractedComponent) "0, 0, 0" false "None")
          (Transformation|SetWorldLocation (LocalVariables|GetAttractedComponent) (Transformation|GetActorLocation) false true)
          (else
            (Physics|AddForce (LocalVariables|GetAttractedComponent) (* (Math|Vector|Normalize _output_get_2) (Variables|InputParameters|GetAttractionFoce)) "None" false)))))))