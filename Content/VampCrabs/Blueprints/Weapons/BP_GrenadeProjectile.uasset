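; Grenade projectile actor that turns into a gravity field shortly after it spawns.
; On BeginPlay it checks the player character's Aiming flag and does nothing further if the player is aiming.
; Otherwise it waits briefly, disables physics and collision on its Cylinder, spawns a scaled-down BP_GravityField at that location and destroys itself.
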(event EventBeginPlay
  (bind _cylinder (Variables|Default|GetCylinder))
  (bind _asbp_character (Utilities|Casting|CastToBP_Character (Game|GetPlayerCharacter 0)))
  (if (not (Variables|/Game/VampCrabs/Blueprints/core/BP_Character.BP_Character_C|GetbAiming _asbp_character))
    (Utilities|FlowControl|Delay 1.0)
    (Physics|SetSimulatePhysics _cylinder false)
    (Collision|SetCollisionEnabled _cylinder "NoCollision")
    (Game|SpawnActorfromClass "/Game/VampCrabs/Blueprints/Weapons/BP_GravityField.BP_GravityField_C" (Math|Transform|MakeTransform (Transformation|GetWorldLocation (Variables|Default|GetCylinder)) "0, 0, 0" "0.100000,0.100000,0.100000") "Undefined" "MultiplyWithRoot" 0 0)
    (Actor|DestroyActor self)))

(fn ConstructionScript)