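; BP_CrabHiveCore is a damageable crab hive enemy that spawns crab swarms and is destroyed when its health runs out.
; While the player is within range, Tick counts BP_CrabBasic actors tagged Wave_Hive, using a DoOnce to spawn gravity-free, tagged batches nearby when none remain.
; Damage lowers health and plays a Niagara effect, while the player overlap only casts.
; Force-based ToPlayer and Group movement functions are defined but not called here.
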(event OnComponentBeginOverlap(Sphere)
  (params (OverlappedComponent :type Primitive%20Component%20Object%20Reference) (OtherActor :type Actor%20Object%20Reference) (OtherComp :type Primitive%20Component%20Object%20Reference) (OtherBodyIndex :type Integer) (bFromSweep :type Boolean) (SweepResult :type Hit%20Result%20Structure%20%28by%20ref%29))
  ;[0.15 0.15 0.15 0.5] DAMAGE PLAYER
  (Utilities|Casting|CastToBP_Character OtherActor))

(event Custom|OnTakeAnyDamage_Event
  (params (DamagedActor :type Actor%20Object%20Reference) (Damage :type Float%20%28single-precision%29) (DamageType :type Damage%20Type%20Object%20Reference) (InstigatedBy :type Controller%20Object%20Reference) (DamageCauser :type Actor%20Object%20Reference))
  ;[0.15 0.15 0.15 0.5] TAKE DAMAGE
  (Variables|Default|SetHealth (- (Variables|Default|GetHealth) Damage))
  (Niagara|SpawnSystemAttached "/Game/VampCrabs/Niagara/NS_Damage.NS_Damage" (Variables|Default|Getcollision) "None" "0.000000,0.000000,20.000000" "0, 0, 0" "KeepRelativeOffset" true))

(event EventToggleGravity
  (params (hasGravuty :type Boolean))
  (bind _crab (Variables|Default|GetCrab))
  ;[0.15 0.15 0.15 0.5] GRAVITY
  (if hasGravuty
    (Physics|SetEnableGravity _crab true)
    (else
      (Physics|SetEnableGravity _crab false))))

(event EventBeginPlay
  (bind _returnvalue (Transformation|GetActorLocation))
  ;[0.15 0.15 0.15 0.5] INIT
  (EventDispatchers|BindEventtoOnTakeAnyDamage (delegate Custom|OnTakeAnyDamage_Event))
  (bind _asbp_character (Utilities|Casting|CastToBP_Character (Game|GetPlayerCharacter 0)))
  (Variables|Default|Setchar _asbp_character)
  (Variables|Default|SetMoveToPlayerSpeed (Math|Random|RandomFloatinRange 1e+02 2e+02))
  (Variables|Default|SetDirectionToDrift (Math|Vector|Normalize (- (Transformation|GetActorLocation (Variables|Default|Getchar)) _returnvalue) 0.001))
  (Transformation|SetWorldRotation (Variables|Default|GetCrab) (Math|Rotator|FindLookatRotation _returnvalue (Transformation|GetActorLocation (Variables|Default|Getchar))) false true))

(event EventTick
  (params (DeltaSeconds :type Float%20%28single-precision%29))
  ;[0.15 0.15 0.15 0.5] Is Dead?
  (if (<= (Variables|Default|GetHealth) 0.0)
    (Actor|DestroyActor)
    (else
      (Utilities|FlowControl|Sequence
        (:then_1
          (Math|Float|CompareFloat (Math|Vector|VectorLength (- (Transformation|GetActorLocation (Variables|Default|Getchar)) (Transformation|GetActorLocation))) (Variables|Default|GetTooFar)
            (:==
              _)
            (:<
              _))
          (bind _outactors (Actor|GetAllActorsOfClasswithTag "/Game/VampCrabs/Blueprints/ENEMIES/BP_CrabBasic.BP_CrabBasic_C" "Wave_Hive"))
          (Math|Integer|CompareInt (Utilities|Array|Length _outactors) 1
            (:==
              (goto _label Reset))
            (:<
              (Utilities|FlowControl|DoOnce false :!label _label
                (:Completed
                  (for _index (range 0 5)
                    (bind _returnvalue (Game|SpawnActorfromClass "/Game/VampCrabs/Blueprints/ENEMIES/BP_CrabBasic.BP_CrabBasic_C" (Math|Transform|MakeTransform (+ (* (Math|Random|RandomUnitVector) (Math|Random|RandomFloatinRange 1e+02 1e+03)) (Transformation|GetActorLocation)) "0, 0, 0" "1.000000,1.000000,1.000000") "AdjustIfPossibleButDontSpawnIfColliding" "MultiplyWithRoot" 0 0))
                    (Utilities|IsValid _returnvalue
                      (:Is%20Valid
                        (Default|ToggleGravity _returnvalue false)
                        (Variables|/Script/Engine.Actor|SetTags _returnvalue (Variables|Default|GetHive%20Tag))))))))))))))

(fn ConstructionScript)

(fn ToPlayer
  (Physics|AddForce (Variables|Default|GetCrab) (* (Variables|Default|GetMoveToPlayerSpeed) (Variables|Default|GetDirectionToDrift)) "None" true)
  (bind _output_get (Variables|Default|SetDirectionToDrift (Math|Vector|Normalize (- (Transformation|GetActorLocation (Variables|Default|Getchar)) (Transformation|GetActorLocation)) 1e-05)))
  (Class|PrimitiveComponent|AddTorqueinRadians (Variables|Default|GetCrab) (Math|Vector|MakeVector 0.0 (.y (Math|Vector|CrossProduct _output_get (Math|Vector|GetRightVector (Variables|Default|GetCrab)))) (.z (Math|Vector|CrossProduct _output_get (Math|Vector|GetRightVector (Variables|Default|GetCrab))))) "None" true))

(fn Group
  (bind _outactors (Actor|GetAllActorsOfClasswithTag "/Game/VampCrabs/Blueprints/ENEMIES/BP_CrabBasic.BP_CrabBasic_C" (Utilities|Array|Get(acopy) (Variables|Actor|GetTags))))
  (for _array_element _outactors
    (Math|Float|CompareFloat (Math|Vector|VectorLength (- (Transformation|GetActorLocation _array_element) (Transformation|GetActorLocation))) (Variables|Default|GetCrabSearchRadius)
      (:==
        _)
      (:<
        _))
    (bind _output_get (Variables|Default|SetDirectionToDrift (Math|Vector|Normalize (- (Transformation|GetActorLocation _array_element) (Transformation|GetActorLocation)))))
    (Physics|AddForce (Variables|Default|GetCrab) (* (Variables|Default|GetMoveToPlayerSpeed) _output_get) "None" true)))