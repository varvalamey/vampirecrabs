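; BP_SniperShot is an enemy homing projectile that damages the player character.
; On spawn it targets the player's capsule through ProjectileMovement, zeroes homing acceleration after two seconds, and destroys itself a second later.
; Any sphere hit stops its movement, but only a BP_Character hit applies fixed damage and destroys it immediately.
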(event OnComponentHit(Sphere)
  (params (HitComponent :type Primitive%20Component%20Object%20Reference) (OtherActor :type Actor%20Object%20Reference) (OtherComp :type Primitive%20Component%20Object%20Reference) (NormalImpulse :type Vector :default "0, 0, 0") (Hit :type Hit%20Result%20Structure%20%28by%20ref%29))
  (Components|Movement|StopMovementImmediately (Variables|Default|GetProjectileMovement))
  (Variables|Default|SetOther_Component HitComponent)
  (bind _output_get (Variables|Default|SetHit_Actor OtherActor))
  (bind _asbp_character (Utilities|Casting|CastToBP_Character _output_get))
  (Game|Damage|ApplyDamage _asbp_character 5e+01 0 0)
  (Actor|DestroyActor))

(event EventBeginPlay
  (bind _projectilemovement (Variables|Default|GetProjectileMovement))
  (bind _asbp_character (Utilities|Casting|CastToBP_Character (Game|GetPlayerCharacter 0)))
  (Variables|/Script/Engine.ProjectileMovementComponent|SetHomingTargetComponent _projectilemovement (Variables|/Script/Engine.Character|GetCapsuleComponent _asbp_character))
  (Utilities|FlowControl|Delay 2.0)
  (Variables|/Script/Engine.ProjectileMovementComponent|SetHomingAccelerationMagnitude _projectilemovement 0.0)
  (Utilities|FlowControl|Delay 1.0)
  (Actor|DestroyActor))

(fn ConstructionScript)