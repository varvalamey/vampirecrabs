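; BP_BasicCrab is a physics-driven crab enemy that homes in on the player, damages them on contact and destroys itself when its health runs out.
; Each tick it pushes its Cube along the direction to the player and applies cross-product torque to turn it.
; Hitting the player or taking damage briefly zeroes the push, then rerolls a random speed, faster after damage.
; A ToggleGravity event switches the Cube's gravity.
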(event OnComponentBeginOverlap(hitbox)
  (params (OverlappedComponent :type Primitive%20Component%20Object%20Reference) (OtherActor :type Actor%20Object%20Reference) (OtherComp :type Primitive%20Component%20Object%20Reference) (OtherBodyIndex :type Integer) (bFromSweep :type Boolean) (SweepResult :type Hit%20Result%20Structure%20%28by%20ref%29))
  (bind _asbp_character (Utilities|Casting|CastToBP_Character OtherActor))
  (Game|Damage|ApplyDamage _asbp_character 1e+01 0 0)
  (Variables|Default|SetMoveToPlayerSpeed 0.0)
  (Utilities|FlowControl|Delay 3.0)
  (Variables|Default|SetMoveToPlayerSpeed (Math|Random|RandomFloatinRange 1e+02 2e+02)))

(event Custom|OnTakeAnyDamage_Event
  (params (DamagedActor :type Actor%20Object%20Reference) (Damage :type Float%20%28single-precision%29) (DamageType :type Damage%20Type%20Object%20Reference) (InstigatedBy :type Controller%20Object%20Reference) (DamageCauser :type Actor%20Object%20Reference))
  (Variables|Default|SetHealth (- (Variables|Default|GetHealth) Damage))
  (Variables|Default|SetMoveToPlayerSpeed 0.0)
  (Utilities|FlowControl|Delay 1.0)
  (Variables|Default|SetMoveToPlayerSpeed (Math|Random|RandomFloatinRange 2e+02 3e+02)))

(event EventToggleGravity
  (params (hasGravuty :type Boolean))
  (bind _cube (Variables|Default|GetCube))
  ;[0.15 0.15 0.15 0.5] GRAVITY
  (if hasGravuty
    (Physics|SetEnableGravity _cube true)
    (else
      (Physics|SetEnableGravity _cube false))))

(event EventBeginPlay
  (EventDispatchers|BindEventtoOnTakeAnyDamage (delegate Custom|OnTakeAnyDamage_Event))
  (bind _asbp_character (Utilities|Casting|CastToBP_Character (Game|GetPlayerCharacter 0)))
  (Variables|Default|Setchar _asbp_character)
  (Variables|Default|SetMoveToPlayerSpeed (Math|Random|RandomFloatinRange 1e+02 2e+02))
  (Variables|Default|Setdirection (Math|Vector|Normalize (- (Transformation|GetActorLocation (Variables|Default|Getchar)) (Transformation|GetActorLocation)) 0.001)))

(event EventTick
  (params (DeltaSeconds :type Float%20%28single-precision%29))
  (if (<= (Variables|Default|GetHealth) 0.0)
    (Actor|DestroyActor)
    (else
      (Physics|AddForce (Variables|Default|GetCube) (* (Variables|Default|GetMoveToPlayerSpeed) (Variables|Default|Getdirection)) "None" true)
      (bind _output_get (Variables|Default|Setdirection (Math|Vector|Normalize (- (Transformation|GetActorLocation (Variables|Default|Getchar)) (Transformation|GetActorLocation)) 1e-05)))
      (Class|PrimitiveComponent|AddTorqueinRadians (Variables|Default|GetCube) (Math|Vector|MakeVector 0.0 (.y (Math|Vector|CrossProduct _output_get (Math|Vector|GetRightVector (Variables|Default|GetCube)))) (.z (Math|Vector|CrossProduct _output_get (Math|Vector|GetRightVector (Variables|Default|GetCube))))) "None" true))))

(fn ConstructionScript)