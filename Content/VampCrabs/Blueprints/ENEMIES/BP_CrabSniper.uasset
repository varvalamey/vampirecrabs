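; BP_CrabSniper is a physics-driven crab enemy that periodically fires a sniper shot and is destroyed when its health runs out.
; Tick uses a timer remainder and DoOnce to spawn BP_SniperShot every five seconds, with collision ignores between shot and shooter.
; Damage lowers health and pauses movement speed for a second before re-randomizing it.
; ToPlayer applies force and cross-product torque toward the player, but this file never calls it.
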(event OnComponentBeginOverlap(hitbox)
  (params (OverlappedComponent :type Primitive%20Component%20Object%20Reference) (OtherActor :type Actor%20Object%20Reference) (OtherComp :type Primitive%20Component%20Object%20Reference) (OtherBodyIndex :type Integer) (bFromSweep :type Boolean) (SweepResult :type Hit%20Result%20Structure%20%28by%20ref%29))
  ;[0.15 0.15 0.15 0.5] DAMAGE PLAYER
)

(event Custom|OnTakeAnyDamage_Event
  (params (DamagedActor :type Actor%20Object%20Reference) (Damage :type Float%20%28single-precision%29) (DamageType :type Damage%20Type%20Object%20Reference) (InstigatedBy :type Controller%20Object%20Reference) (DamageCauser :type Actor%20Object%20Reference))
  ;[0.15 0.15 0.15 0.5] TAKE DAMAGE
  (Variables|Default|SetHealth (- (Variables|Default|GetHealth) Damage))
  (Variables|Default|SetMoveToPlayerSpeed 0.0)
  (Utilities|FlowControl|Delay 1.0)
  (Variables|Default|SetMoveToPlayerSpeed (Math|Random|RandomFloatinRange 2e+02 3e+02)))

(event EventToggleGravity
  (params (hasGravuty :type Boolean))
  (bind _cube (Variables|Default|GetCube))
  ;[0.15 0.15 0.15 0.5] GRAVITY
  (if hasGravuty
    (Physics|SetEnableGravity _cube true)
    (else
      (Physics|SetEnableGravity _cube false))))

(event EventBeginPlay
  ;[0.15 0.15 0.15 0.5] INIT
  (EventDispatchers|BindEventtoOnTakeAnyDamage (delegate Custom|OnTakeAnyDamage_Event)))

(event EventTick
  (params (DeltaSeconds :type Float%20%28single-precision%29))
  (bind _cube (Variables|Default|GetCube))
  (bind _returnvalue (Transformation|GetWorldTransform _cube))
  ;[0.15 0.15 0.15 0.5] Is Dead?
  (Variables|Default|Settimer (+ (Variables|Default|Gettimer) DeltaSeconds))
  (if (<= (Variables|Default|GetHealth) 0.0)
    (Actor|DestroyActor)
    (else
      (Math|Float|CompareFloat (.Remainder (Math|Float|Division(WholeandRemainder) (Variables|Default|Gettimer) 5.0)) 0.1
        (:>
          (goto _label Reset))
        (:==
          _)
        (:<
          _))
      (Utilities|FlowControl|DoOnce false :!label _label
        (:Completed
          (bind _returnvalue_2 (Game|SpawnActorfromClass "/Game/VampCrabs/Blueprints/ENEMIES/BP_SniperShot.BP_SniperShot_C" (Math|Transform|MakeTransform (+ (.location _returnvalue) 5e+01) (.rotation _returnvalue) (.scale _returnvalue)) "AlwaysSpawn" "MultiplyWithRoot" 0 0))
          ;[1 1 1 1 11] bullet collision
          (Collision|IgnoreActorwhenMoving (Variables|Default|GetCube) _returnvalue_2 true)
          (Collision|IgnoreActorwhenMoving (Variables|/Game/VampCrabs/Blueprints/ENEMIES/BP_SniperShot.BP_SniperShot_C|GetSphere _returnvalue_2) self true))))))

(fn ConstructionScript)

(fn ToPlayer
  (Physics|AddForce (Variables|Default|GetCube) (* (Variables|Default|GetMoveToPlayerSpeed) (Variables|Default|GetDirectionToPlayer)) "None" true)
  (bind _output_get (Variables|Default|SetDirectionToPlayer (Math|Vector|Normalize (- (Transformation|GetActorLocation (Variables|Default|Getchar)) (Transformation|GetActorLocation)) 1e-05)))
  (Class|PrimitiveComponent|AddTorqueinRadians (Variables|Default|GetCube) (Math|Vector|MakeVector 0.0 (.y (Math|Vector|CrossProduct _output_get (Math|Vector|GetRightVector (Variables|Default|GetCube)))) (.z (Math|Vector|CrossProduct _output_get (Math|Vector|GetRightVector (Variables|Default|GetCube))))) "None" true))